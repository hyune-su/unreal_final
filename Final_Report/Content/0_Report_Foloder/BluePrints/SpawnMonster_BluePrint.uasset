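; A monster spawner actor that creates a limited number of AI monsters at its own location and rotation.
; Tick increments a frame-based timer, so the spawn interval depends on frame rate rather than seconds.
; Each time the timer reaches its threshold, it spawns MonsterBluePrint, resets the timer and increments a count.
; Once five spawn attempts are counted, the spawner destroys itself on the following tick.
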(event EventTick
  (params (DeltaSeconds :type Float%20%28single-precision%29))
  (bind _result (Math|Float|IncrementFloat (Variables|Default|GetTimer))
    (:%20%20
      (if (== (Variables|Default|GetCount) 5)
        (Actor|DestroyActor)
        (elif (>= (Math|Float|Truncate _result) 600)
          (AI|SpawnAIFromClass "/Game/0_Report_Foloder/Character/MonsterBluePrint.MonsterBluePrint_C" 0 (Transformation|GetActorLocation) (Transformation|GetActorRotation) false)
          (Variables|Default|SetTimer 0.0)
          (Math|Integer|IncrementInt (Variables|Default|GetCount)))))))

(fn ConstructionScript)
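; Fire trap actor that stays hidden until the player comes within a short range, then damages whoever stands in it.
; Tick checks distance to the living player to toggle visibility, applying damage every frame while the capsule overlap flag is set and the player is in range.
; Incoming damage lowers the trap's HP, and reaching exactly zero plays a sound at the world origin and destroys it.
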(event OnComponentEndOverlap(Capsule)
  (params (OverlappedComponent :type Primitive%20Component%20Object%20Reference) (OtherActor :type Actor%20Object%20Reference) (OtherComp :type Primitive%20Component%20Object%20Reference) (OtherBodyIndex :type Integer))
  (Variables|Default|SetisOverlap false))

(event OnComponentBeginOverlap(Capsule)
  (params (OverlappedComponent :type Primitive%20Component%20Object%20Reference) (OtherActor :type Actor%20Object%20Reference) (OtherComp :type Primitive%20Component%20Object%20Reference) (OtherBodyIndex :type Integer) (bFromSweep :type Boolean) (SweepResult :type Hit%20Result%20Structure%20%28by%20ref%29))
  (Variables|Default|SetisOverlap true)
  (bind _asplayer_character (Utilities|Casting|CastToPlayerCharacter OtherActor)))

(event EventBeginPlay
  (Rendering|SetActorHiddenInGame true)
  (bind _returnvalue (Actor|GetActorOfClass "/Game/0_Report_Foloder/Character/PlayerCharacter.PlayerCharacter_C")))

(event EventTick
  (params (DeltaSeconds :type Float%20%28single-precision%29))
  (bind _isoverlap (Variables|Default|GetisOverlap))
  (if (not (Variables|/Game/0_Report_Foloder/Character/PlayerCharacter.PlayerCharacter_C|GetIsDeath (stale EventBeginPlay _returnvalue)))
    (if _isoverlap
      _
      (else
        _))
    (if (<= (Math|Vector|VectorLength (- (Transformation|GetActorLocation) (Transformation|GetActorLocation (stale EventBeginPlay _returnvalue)))) 3e+02)
      (Rendering|SetActorHiddenInGame false)
      (if _isoverlap
        (Game|Damage|ApplyDamage (stale OnComponentBeginOverlap(Capsule) _asplayer_character) (Variables|Default|GetDamage) 0 0))
      (else
        (Variables|Default|SetisSound false)
        (Rendering|SetActorHiddenInGame true)))))

(event Game|Damage|EventAnyDamage
  (params (Damage :type Float%20%28single-precision%29) (DamageType :type Damage%20Type%20Object%20Reference) (InstigatedBy :type Controller%20Object%20Reference) (DamageCauser :type Actor%20Object%20Reference))
  (bind _output_get (Variables|Default|SetTrap_Hp (- (Variables|Default|GetTrap_Hp) Damage)))
  (if (== _output_get 0.0)
    (Audio|PlaySoundatLocation "/Engine/EditorSounds/Notifications/CompileFailed_Cue.CompileFailed_Cue" "0, 0, 0" "0, 0, 0" 1.0 1.0 0.0 0 0 0)
    (Actor|DestroyActor)))

(fn ConstructionScript)